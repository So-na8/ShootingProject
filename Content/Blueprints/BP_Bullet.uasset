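; BP_Bullet is a projectile that destroys BP_Enemy actors on contact and awards score.
; Tick moves it along its forward vector at MoveSpeed, scaled by delta time, without sweeping.
; On overlap with an enemy, it destroys both actors, spawns an explosion particle at its location and adds a point through BP_GameModeBase.
; DestroyActor is called on the bullet both before the effect and score steps and again after them.
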(event `self.ReceiveActorBeginOverlap`
  (params (OtherActor :type "Actor Object Reference"))
  (bind _asbp_enemy (cast `/Game/Blueprints/BP_Enemy` OtherActor))
  (`self.K2_DestroyActor` _asbp_enemy)
  (`self.K2_DestroyActor`)
  (`GameplayStatics.SpawnEmitterAtLocation` "/Game/StarterContent/Particles/P_Explosion.P_Explosion" (`self.K2_GetActorLocation`))
  (bind _asbp_game_mode_base (cast `/Game/Blueprints/BP_GameModeBase` (`GameplayStatics.GetGameMode`)))
  (`/Game/Blueprints/BP_GameModeBase.AddScore` _asbp_game_mode_base 1)
  (`self.K2_DestroyActor`))

(event `self.ReceiveTick`
  (params (DeltaSeconds :type "Float (single-precision)"))
  (`self.K2_SetActorLocation` (+ (`self.K2_GetActorLocation`) (* (* (`self.GetActorForwardVector`) (`self.MoveSpeed`)) DeltaSeconds))))

(fn `UserConstructionScript`)